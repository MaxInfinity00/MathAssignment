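; BP_HoverBouncePad is a bounce pad that launches characters upward when they hit it from above.
; On Hit, it compares the normalized direction from the pad to the other actor against world up with a dot product.
; If that actor lies within a cone above the pad and is a Character, it applies a large vertical force through the CharacterMovement component.
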(event EventBeginPlay)

(event Collision|EventActorBeginOverlap
  (params (OtherActor :type Actor%20Object%20Reference)))

(event EventTick
  (params (DeltaSeconds :type Float%20%28single-precision%29)))

(event Collision|EventHit
  (params (MyComp :type Primitive%20Component%20Object%20Reference) (Other :type Actor%20Object%20Reference) (OtherComp :type Primitive%20Component%20Object%20Reference) (bSelfMoved :type Boolean) (HitLocation :type Vector :default "0, 0, 0") (HitNormal :type Vector :default "0, 0, 0") (NormalImpulse :type Vector :default "0, 0, 0") (Hit :type Hit%20Result%20Structure%20%28by%20ref%29))
  (if (> (Math|Vector|DotProduct (Math|Vector|Normalize (- (Transformation|GetActorLocation Other) (Transformation|GetActorLocation))) (Math|Vector|VectorUp)) 0.7)
    (bind _ascharacter (Utilities|Casting|CastToCharacter Other))
    (Physics|AddForce (Variables|/Script/Engine.Character|GetCharacterMovement _ascharacter) "0.000000,0.000000,15000000.000000")))

(fn ConstructionScript)