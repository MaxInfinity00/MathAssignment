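; BP_Pickup is a coin pickup that spins until the third-person character comes within range, then hides.
; While uncollected, Tick rotates the Cylinder about the up axis at RotationSpeed and looks up BP_ThirdPersonCharacter each frame.
; Intersection is tested manually, without overlap events, comparing squared distance (a dot product) to CharacterRange times PickupRange.
; A hit hides the mesh and sets Collected, stopping further rotation and checks.
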(event EventBeginPlay)

(event Collision|EventActorBeginOverlap
  (params (OtherActor :type Actor%20Object%20Reference)))

(event EventTick
  (params (DeltaSeconds :type Float%20%28single-precision%29))
  (if (not (Variables|Default|Getcollected))
    ;[1 1 1] Rotate Coin
    (Transformation|AddWorldRotation (Variables|Default|GetCylinder) (Math|Vector|RotatorfromAxisandAngle (Math|Vector|VectorUp) (* DeltaSeconds (Variables|Default|Getrotation%20speed))) false false)
    ;[1 1 1] Check Intersection
    (bind _returnvalue (Actor|GetActorOfClass "/Game/ThirdPerson/Blueprints/BP_ThirdPersonCharacter.BP_ThirdPersonCharacter_C"))
    (if (<= (Math|Vector|DotProduct (- (Transformation|GetActorLocation _returnvalue) (Transformation|GetActorLocation)) (- (Transformation|GetActorLocation _returnvalue) (Transformation|GetActorLocation))) (* (Variables|Default|GetCharacterRange) (Variables|Default|GetPickup%20Range)))
      (Rendering|SetVisibility (Variables|Default|GetCylinder) false false)
      (Variables|Default|Setcollected true))))

(fn ConstructionScript)